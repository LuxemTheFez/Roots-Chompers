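; Base enemy character Blueprint that holds its stats in an EnemieStruct, handling damage, death, movement speed and stun state.
; Damage lowers the struct's health, and once it would reach zero the enemy destroys itself and adds a point to the score in the BP_GameStorage game instance.
; Stunned and Unstunned events toggle a struct flag, which Tick polls each frame to set walk speed to zero or the struct's speed.
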(event `self.ReceiveBeginPlay`
  (bind (_enemiestruct_type _enemiestruct_health _enemiestruct_speed _enemiestruct_strength _enemiestruct_isstunned) (break `/Game/TopDown/Blueprints/Structure/EnemiesStructure` (`self.EnemieStruct`)))
  (set `CharacterMovementComponent.MaxWalkSpeed` _enemiestruct_speed (`self.CharacterMovement`)))

(event `/Game/Ennemies/I_EnemiesInterface.TakeDamage`
  (params (Damage :type "Float (double-precision)"))
  (bind (_enemiestruct_type _enemiestruct_health _enemiestruct_speed _enemiestruct_strength _enemiestruct_isstunned) (break `/Game/TopDown/Blueprints/Structure/EnemiesStructure` (`self.EnemieStruct`)))
  (bind (_enemiestruct_type_2 _enemiestruct_health_2 _enemiestruct_speed_2 _enemiestruct_strength_2 _enemiestruct_isstunned_2 _enemiestruct_speedmulti _enemiestruct_weight) (break `/Game/TopDown/Blueprints/Structure/EnemiesStructure` (`self.EnemieStruct`)))
  (bind _returnvalue (- _enemiestruct_health Damage))
  (if (> _returnvalue 0.0)
    (set `self.EnemieStruct` (make `/Game/TopDown/Blueprints/Structure/EnemiesStructure` _enemiestruct_type_2 _returnvalue _enemiestruct_speed_2 _enemiestruct_strength_2 _enemiestruct_isstunned_2 _enemiestruct_speedmulti _enemiestruct_weight))
    (else
      (`self.K2_DestroyActor`)
      (bind _asbp_game_storage (cast `/Game/TopDown/Blueprints/BP_GameStorage` (`GameplayStatics.GetGameInstance`)))
      (`/Game/TopDown/Blueprints/BP_GameStorage.AddScore` _asbp_game_storage 1))))

(event `self.ReceiveTick`
  (params (DeltaSeconds :type "Float (single-precision)"))
  (bind (_enemiestruct_type _enemiestruct_health _enemiestruct_speed _enemiestruct_strength _enemiestruct_isstunned) (break `/Game/TopDown/Blueprints/Structure/EnemiesStructure` (`self.EnemieStruct`)))
  (bind _charactermovement (`self.CharacterMovement`))
  (if _enemiestruct_isstunned
    (set `CharacterMovementComponent.MaxWalkSpeed` 0.0 _charactermovement)
    (else
      (set `CharacterMovementComponent.MaxWalkSpeed` _enemiestruct_speed _charactermovement))))

(event `Stunned`
  (bind (_enemiestruct_type _enemiestruct_health _enemiestruct_speed _enemiestruct_strength _enemiestruct_isstunned _enemiestruct_speedmulti _enemiestruct_weight) (break `/Game/TopDown/Blueprints/Structure/EnemiesStructure` (`self.EnemieStruct`)))
  (set `self.EnemieStruct` (make `/Game/TopDown/Blueprints/Structure/EnemiesStructure` _enemiestruct_type _enemiestruct_health _enemiestruct_speed _enemiestruct_strength true _enemiestruct_speedmulti _enemiestruct_weight)))

(event `Unstunned`
  (bind (_enemiestruct_type _enemiestruct_health _enemiestruct_speed _enemiestruct_strength _enemiestruct_isstunned _enemiestruct_speedmulti _enemiestruct_weight) (break `/Game/TopDown/Blueprints/Structure/EnemiesStructure` (`self.EnemieStruct`)))
  (set `self.EnemieStruct` (make `/Game/TopDown/Blueprints/Structure/EnemiesStructure` _enemiestruct_type _enemiestruct_health _enemiestruct_speed _enemiestruct_strength false _enemiestruct_speedmulti _enemiestruct_weight)))

(fn `UserConstructionScript`)