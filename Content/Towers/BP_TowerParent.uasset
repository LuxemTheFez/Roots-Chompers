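; Parent Blueprint for plant towers that automatically attack enemies entering their range.
; A Range sphere, sized from PlantStructure on BeginPlay, adds overlapping I_EnemiesInterface actors to an enemy list and removes them on exit.
; The first arrival starts a looping attack-speed timer that damages the oldest listed enemy and plays either Niagara or mesh animation feedback.
; An empty list clears IsShooting, making ticks idle without stopping the timer.
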(event `Tapoter`
  (bind (_plantstructure_type _plantstructure_range _plantstructure_cost _plantstructure_strength _plantstructure_isstunned _plantstructure_attackspeed _plantstructure_enemieslist) (break `/Game/TopDown/Blueprints/Structure/PlantsStructure` (`self.PlantStructure`)))
  (bind _mesh (`self.Mesh`))
  (if (stale `self.Range.OnComponentBeginOverlap` _output_get)
    (message `/Game/Ennemies/I_EnemiesInterface.TakeDamage` (`|GetArrayItem` _plantstructure_enemieslist) _plantstructure_strength)
    (if (`self.isNS`)
      (`ActorComponent.Activate` (`self.Niagara`) true)
      (elif (`self.isAnimated`)
        (`SkeletalMeshComponent.Play` (`self.Mesh`) false)
        (if (== (`SkeletalMeshComponent.GetPosition` _mesh) 1.0)
          (`SkeletalMeshComponent.SetPosition` _mesh 0.0 true))))))

(event `self.Range.OnComponentBeginOverlap`
  (params (OverlappedComponent :type "PrimitiveComponent Object Reference") (OtherActor :type "Actor Object Reference") (OtherComp :type "PrimitiveComponent Object Reference") (OtherBodyIndex :type Integer) (bFromSweep :type Boolean) (SweepResult :type "HitResult Structure (by ref)"))
  (bind (_plantstructure_type _plantstructure_range _plantstructure_cost _plantstructure_strength _plantstructure_isstunned _plantstructure_attackspeed _plantstructure_enemieslist) (break `/Game/TopDown/Blueprints/Structure/PlantsStructure` (`self.PlantStructure`)))
  (bind (_plantstructure_type_2 _plantstructure_range_2 _plantstructure_cost_2 _plantstructure_strength_2 _plantstructure_isstunned_2 _plantstructure_attackspeed_2 _plantstructure_enemieslist_2) (break `/Game/TopDown/Blueprints/Structure/PlantsStructure` (`self.PlantStructure`)))
  (bind _isshooting (`self.isShooting`))
  (if (`KismetSystemLibrary.DoesImplementInterface` OtherActor "/Game/Ennemies/I_EnemiesInterface.I_EnemiesInterface_C")
    (`KismetArrayLibrary.Array_AddUnique` _plantstructure_enemieslist OtherActor)
    (if _isshooting
      (`KismetSystemLibrary.PrintString` "Je tire déjà" true true (struct :`R` 1.0 :`G` 0.152418 :`B` 0.102654 :`A` 1.0))
      (else
        (bind _output_get (set `self.isShooting` (not _isshooting)))
        (`KismetSystemLibrary.K2_SetTimerDelegate` (delegate `Tapoter`) _plantstructure_attackspeed_2 true)))))

(event `self.Range.OnComponentEndOverlap`
  (params (OverlappedComponent :type "PrimitiveComponent Object Reference") (OtherActor :type "Actor Object Reference") (OtherComp :type "PrimitiveComponent Object Reference") (OtherBodyIndex :type Integer))
  (bind (_plantstructure_type _plantstructure_range _plantstructure_cost _plantstructure_strength _plantstructure_isstunned _plantstructure_attackspeed _plantstructure_enemieslist) (break `/Game/TopDown/Blueprints/Structure/PlantsStructure` (`self.PlantStructure`)))
  (`KismetArrayLibrary.Array_RemoveItem` _plantstructure_enemieslist OtherActor)
  (if (== (`KismetArrayLibrary.Array_Length` _plantstructure_enemieslist) 0)
    (set `self.isShooting` false)))

(event `self.ReceiveBeginPlay`
  (bind (_plantstructure_type _plantstructure_range _plantstructure_cost _plantstructure_strength _plantstructure_isstunned _plantstructure_attackspeed _plantstructure_enemieslist) (break `/Game/TopDown/Blueprints/Structure/PlantsStructure` (`self.PlantStructure`)))
  (`SphereComponent.SetSphereRadius` (`self.Range`) _plantstructure_range true))

(fn `UserConstructionScript`)