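; BP_Stunner is a plant tower that stuns enemies, extending a parent tower Blueprint and setting a spore Niagara effect and animated flag on BeginPlay.
; Each Tick it takes the first enemy in PlantStructure's EnemiesList, stuns it if it differs from the last one stunned, and unstuns it after a three-second Delay.
; Petal animation playback and a debug print remain as unconnected nodes.
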(event `self.ReceiveBeginPlay`
  (`parent.ReceiveBeginPlay`)
  (set `self.Niagara` (`self.Spore`))
  (set `self.isAnimated` true))

(event `self.ReceiveTick`
  (params (DeltaSeconds :type "Float (single-precision)"))
  (bind (_plantstructure_type _plantstructure_range _plantstructure_cost _plantstructure_strength _plantstructure_isstunned _plantstructure_attackspeed _plantstructure_enemieslist) (break `/Game/TopDown/Blueprints/Structure/PlantsStructure` (`self.PlantStructure`)))
  (bind _output (`|GetArrayItem` _plantstructure_enemieslist))
  (`/Engine/EditorBlueprintResources/StandardMacros.IsValid` _output
    (:`Is Valid`
      (bind _asbp_ennemi_parent (cast `/Game/Ennemies/Bp_EnnemiParent` _output))
      (if (!= _output (`self.lastStunne`))
        (`/Game/Ennemies/Bp_EnnemiParent.Stunned` _asbp_ennemi_parent)
        (set `self.lastStunne` _output)
        (`KismetSystemLibrary.Delay` 3.0)
        (`/Engine/EditorBlueprintResources/StandardMacros.IsValid` _asbp_ennemi_parent
          (:`Is Valid`
            (`/Game/Ennemies/Bp_EnnemiParent.Unstunned` _asbp_ennemi_parent)))))))

(fn `UserConstructionScript`
  (`parent.UserConstructionScript`))