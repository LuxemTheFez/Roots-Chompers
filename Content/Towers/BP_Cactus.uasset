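; Cactus tower actor that turns to face enemies, built on a parent class that supplies its begin-play and construction logic.
; On begin play it runs the parent logic, then sets its IsNS and IsAnimated flags.
; Each tick, while the first enemy in PlantStructure's list is valid, it rotates toward that enemy.
; It also rewinds the mesh animation whenever playback reaches position 1.0, with notifies enabled.
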(event `self.ReceiveBeginPlay`
  (`parent.ReceiveBeginPlay`)
  (set `self.isNS` false)
  (set `self.isAnimated` true))

(event `self.ReceiveTick`
  (params (DeltaSeconds :type "Float (single-precision)"))
  (bind (_plantstructure_type _plantstructure_range _plantstructure_cost _plantstructure_strength _plantstructure_isstunned _plantstructure_attackspeed _plantstructure_enemieslist) (break `/Game/TopDown/Blueprints/Structure/PlantsStructure` (`self.PlantStructure`)))
  (bind _mesh (`self.Mesh`))
  (bind _output (`|GetArrayItem` _plantstructure_enemieslist))
  (`/Engine/EditorBlueprintResources/StandardMacros.IsValid` _output
    (:`Is Valid`
      (`self.K2_SetActorRotation` (`KismetMathLibrary.FindLookAtRotation` (`self.K2_GetActorLocation`) (`self.K2_GetActorLocation` _output)))
      (if (== (`SkeletalMeshComponent.GetPosition` _mesh) 1.0)
        (`SkeletalMeshComponent.SetPosition` _mesh 0.0 true)))))

(fn `UserConstructionScript`
  (`parent.UserConstructionScript`))