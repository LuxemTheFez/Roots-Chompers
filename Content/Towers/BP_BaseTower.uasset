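; BP_BaseTower is a tower that turns to face and aims a projectile effect at an enemy.
; On BeginPlay it runs the parent logic and stores its Projectile component in the Niagara variable.
; Each Tick, if the first entry in PlantStructure's EnemiesList is valid, it snaps its rotation toward that enemy.
; It also feeds the enemy's location to the Projectile's CiblePosition vector parameter.
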(event `self.ReceiveBeginPlay`
  (`parent.ReceiveBeginPlay`)
  (set `self.Niagara` (`self.Projectile`)))

(event `self.ReceiveTick`
  (params (DeltaSeconds :type "Float (single-precision)"))
  (bind (_plantstructure_type _plantstructure_range _plantstructure_cost _plantstructure_strength _plantstructure_isstunned _plantstructure_attackspeed _plantstructure_enemieslist) (break `/Game/TopDown/Blueprints/Structure/PlantsStructure` (`self.PlantStructure`)))
  (bind _output (`|GetArrayItem` _plantstructure_enemieslist))
  (bind _returnvalue (`self.K2_GetActorLocation` _output))
  (`/Engine/EditorBlueprintResources/StandardMacros.IsValid` _output
    (:`Is Valid`
      (`self.K2_SetActorRotation` (`KismetMathLibrary.FindLookAtRotation` (`self.K2_GetActorLocation`) _returnvalue))
      (`FXSystemComponent.SetVectorParameter` (`self.Projectile`) "CiblePosition" _returnvalue))))

(fn `UserConstructionScript`
  (`parent.UserConstructionScript`))